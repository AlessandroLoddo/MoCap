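; Holdable magic wand prop that fires a BP_Projectile automatically while gripped and held roughly level.
; Grip and drop events toggle ticking, and each tick checks mesh pitch and cooldown before spawning at the Scene component and launching along mesh forward via physics velocity.
; A shot resets the cooldown timer, which later non-firing ticks count down, but the timer comparison in InCooldown is left unused.
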(event `/Game/Blueprints/HoldableProps/GrippableInterface.OnDropped`
  (`parent.OnDropped`)
  (set `self.bIsGripped` false)
  (`self.SetActorTickEnabled` false))

(event `/Game/Blueprints/HoldableProps/GrippableInterface.OnGripped`
  (`parent.OnGripped`)
  (set `self.bIsGripped` true)
  (`self.SetActorTickEnabled` true))

(event `self.ReceiveTick`
  (params (DeltaSeconds :type "Float (single-precision)"))
  (if (`self.bIsGripped`)
    ;[0.2697 0.06412 1] Check rotation
    (bind _isinshootingrotation (`self.IsInShootingRotation`))
    (if _isinshootingrotation
      ;[1 0.0245 0.1342] Check cooldown
      (if (`self.InCooldown`)
        (`self.UpdateCooldown` :!label _label)
        (else
          ;[1 0.271 0] Shooting implementation
          (bind _returnvalue (`|SpawnActorFromClass` "/Game/Blueprints/HoldableProps/BP_Projectile.BP_Projectile_C" (`KismetMathLibrary.MakeTransform` (`SceneComponent.K2_GetComponentLocation` (`self.Scene`))) "Undefined" "MultiplyWithRoot" null null))
          (`PrimitiveComponent.SetPhysicsLinearVelocity` (`/Game/Blueprints/HoldableProps/BP_Projectile.Sphere` _returnvalue) (* (`SceneComponent.GetForwardVector` (`self.GrippableObjectMesh`)) (`self.ProjectileSpeed`)) false "None")
          (set `self.CooldownTimer` 3.0)
          (set `self.bIsInCooldown` true)))
      (else
        (goto _label)))))

(fn `IsInShootingRotation`
  (returns (IsInShootingRotation :type Boolean))
  (bind (_returnvalue_roll _returnvalue_pitch) (`KismetMathLibrary.BreakRotator` (`SceneComponent.K2_GetComponentRotation` (`self.GrippableObjectMesh`))))
  (if (and (< _returnvalue_pitch 15.0) (> _returnvalue_pitch -15.0))
    (return true)
    (else
      (return false))))

(fn `UpdateCooldown`
  (set `self.CooldownTimer` (- (`self.CooldownTimer`) (`GameplayStatics.GetWorldDeltaSeconds`))))

(fn `UserConstructionScript`
  (`parent.UserConstructionScript`))