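; BP_RollingSphere is a physics golf ball that detects when it comes to rest and whether it landed in the goal.
; Overlap with a BP_GolfClub passes a DoOnce gate and starts a delayed polling loop until velocity is near zero.
; It then checks for BP_GolfGoal overlap, calls GolfGoalReached or UpdateBall, and re-arms the gate.
; ResetBall returns it to its BeginPlay position and clears its velocity.
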(event `self.ReceiveBeginPlay`
  (set `self.StartingPos` (`SceneComponent.K2_GetComponentLocation` (`self.Sphere`))))

(event `ResetBall`
  (bind _sphere (`self.Sphere`))
  ;[1 0.2823 0.7028] Reset Ball
  (`SceneComponent.K2_SetWorldLocation` _sphere (`self.StartingPos`) false false)
  (`PrimitiveComponent.SetPhysicsLinearVelocity` _sphere (0.0 0.0 0.0) false "None")
  (`PrimitiveComponent.SetAllPhysicsAngularVelocityInDegrees` _sphere (0.0 0.0 0.0) false))

(event `IsInGoalEvent`
  ;[1 0.5332 0.1223] After the ball hits the club, after some time, check whether the ball is in the goal or not
  (if (`KismetArrayLibrary.Array_IsNotEmpty` (`PrimitiveComponent.GetOverlappingActors` (`self.SphereCollision`) "/Game/Blueprints/HoldableProps/Golf/BP_GolfGoal.BP_GolfGoal_C"))
    (`self.GolfGoalReached`)
    (goto _label :!via `Reset`)
    (else
      (`self.UpdateBall`)
      (goto _label :!via `Reset`))))

(event `self.SphereCollision.OnComponentBeginOverlap`
  (params (OverlappedComponent :type "PrimitiveComponent Object Reference") (OtherActor :type "Actor Object Reference") (OtherComp :type "PrimitiveComponent Object Reference") (OtherBodyIndex :type Integer) (bFromSweep :type Boolean) (SweepResult :type "HitResult Structure (by ref)"))
  ;[0.4686 0.1165 1] Once ball overlaps club, check its speed until its low enough, check then if it is in the goal
  (cast `/Game/Blueprints/HoldableProps/Golf/BP_GolfClub` OtherActor)
  (`/Engine/EditorBlueprintResources/StandardMacros.DoOnce` false :!label _label
    (:`Completed`
      (`KismetSystemLibrary.Delay` 1.0 :!label _label_2)
      (if (< (`KismetMathLibrary.VSize` (`SceneComponent.GetComponentVelocity` (`self.Sphere`))) 4.0)
        (`self.IsInGoalEvent`)
        (else
          (`KismetSystemLibrary.Delay` 0.6)
          (goto _label_2))))))

(fn `UserConstructionScript`)