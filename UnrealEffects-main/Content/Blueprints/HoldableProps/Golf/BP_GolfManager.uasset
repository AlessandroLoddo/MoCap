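; Manager actor for a golf minigame that coordinates the ball, goal, decorations and camera.
; On each ball update it resets the ball and shifts the goal and decorations opposite or relative to the ball's displacement, so the course moves instead of the ball's origin.
; When the goal is reached, the hole flashes green, relocates to a random navigable point, and the ball resets and turns toward it with the camera placed behind.
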(event `UpdateOnGoalReached`
  ;[1 1 1] Goal has been reached by ball, delay and then change color, reset ball
  (`MeshComponent.SetVectorParameterValueOnMaterials` (`/Game/Blueprints/HoldableProps/Golf/BP_GolfGoal.Hole` (`self.GolfGoal`)) "Color" (0.0 1.0 0.0))
  (`KismetSystemLibrary.Delay` 2.0)
  (`MeshComponent.SetVectorParameterValueOnMaterials` (`/Game/Blueprints/HoldableProps/Golf/BP_GolfGoal.Hole` (`self.GolfGoal`)) "Color" (0.0 1.0 0.87))
  (`SceneComponent.K2_SetWorldLocation` (`Actor.RootComponent` (`self.GolfGoal`)) (`NavigationSystemV1.K2_GetRandomReachablePointInRadius` (0.0 0.0 -24.041572) 1500.0 null null) false false)
  (`/Game/Blueprints/HoldableProps/Golf/BP_RollingSphere.ResetBall` (`self.GolfBall`))
  (`self.CameraTowardsBallMove`))

(event `CameraTowardsBallMove`
  (bind _sphere (`/Game/Blueprints/HoldableProps/Golf/BP_RollingSphere.Sphere` (`self.GolfBall`)))
  (bind (_returnvalue_roll _returnvalue_pitch _returnvalue_yaw) (`KismetMathLibrary.BreakRotator` (`KismetMathLibrary.FindLookAtRotation` (`SceneComponent.K2_GetComponentLocation` _sphere) (`SceneComponent.K2_GetComponentLocation` (`/Game/Blueprints/HoldableProps/Golf/BP_GolfGoal.Hole` (`self.GolfGoal`))))))
  ;[1 0.2834 0.1603] Set golf ball to rotate towards golf hole
  (`SceneComponent.K2_SetWorldRotation` _sphere (`KismetMathLibrary.MakeRotator` 0.0 _returnvalue_pitch _returnvalue_yaw) false false)
  ;[0.8177 0.2393 1] Set camera to look at golf hole
  (`self.ApplyCameraOffset`))

(event `self.ReceiveBeginPlay`
  (bind _golfball (`self.GolfBall`))
  (bind (_returnvalue_x _returnvalue_y _returnvalue_z) (`KismetMathLibrary.BreakVector` (`SceneComponent.K2_GetComponentLocation` (`/Game/Blueprints/HoldableProps/Golf/BP_GolfGoal.Hole` (`self.GolfGoal`)))))
  (`self.SetAllGolfDecorations`)
  (add `/Game/Blueprints/HoldableProps/Golf/BP_RollingSphere.GolfGoalReached` _golfball (delegate `UpdateOnGoalReached`))
  (add `/Game/Blueprints/HoldableProps/Golf/BP_RollingSphere.UpdateBall` _golfball (delegate `UpdateGoalAndBall`))
  (set `self.StartingHeight` _returnvalue_z)
  (`/Game/Blueprints/HoldableProps/Golf/BP_RollingSphere.UpdateBall` (`self.GolfBall`)))

(event `UpdateGoalAndBall`
  (bind _golfgoal (`self.GolfGoal`))
  (bind (_returnvalue_x _returnvalue_y) (`KismetMathLibrary.BreakVector` (+ (`SceneComponent.K2_GetComponentLocation` (`Actor.RootComponent` _golfgoal)) (* (`self.UpdatePos`) -1.0))))
  ;[0.607 1 0.2736] Move goal depending on where ball was, then reset ball and move camera towards goal behind ball
  (`self.GetBallDisplacement`)
  (`SceneComponent.K2_SetWorldLocation` (`Actor.RootComponent` _golfgoal) (`KismetMathLibrary.MakeVector` _returnvalue_x _returnvalue_y (`self.StartingHeight`)) false false)
  (`/Game/Blueprints/HoldableProps/Golf/BP_RollingSphere.ResetBall` (`self.GolfBall`))
  (`self.OffsetAllDecorations`))

(fn `ApplyCameraOffset`
  (bind _sphere (`/Game/Blueprints/HoldableProps/Golf/BP_RollingSphere.Sphere` (`self.GolfBall`)))
  (bind _returnvalue (`SceneComponent.K2_GetComponentLocation` _sphere))
  (bind (_returnvalue_x _returnvalue_y _returnvalue_z) (`KismetMathLibrary.BreakVector` (+ _returnvalue (/ 1000.0 4.0))))
  (bind (_returnvalue_x_2 _returnvalue_y_2) (`KismetMathLibrary.BreakVector` (+ _returnvalue (* (* (`SceneComponent.GetForwardVector` _sphere) -1.0) 400.0))))
  (`SceneComponent.K2_SetWorldLocation` (`/Game/Blueprints/BP_MoCapPawn.Camera` (`self.MyPawn`)) (`KismetMathLibrary.MakeVector` _returnvalue_x_2 _returnvalue_y_2 _returnvalue_z) false false))

(fn `GetBallDisplacement`
  (bind _golfball (`self.GolfBall`))
  (bind _returnvalue (- (`SceneComponent.K2_GetComponentLocation` (`/Game/Blueprints/HoldableProps/Golf/BP_RollingSphere.Sphere` _golfball)) (`/Game/Blueprints/HoldableProps/Golf/BP_RollingSphere.StartingPos` _golfball)))
  (set `self.UpdatePos` (* (`KismetMathLibrary.Normal` _returnvalue) (`KismetMathLibrary.VSize` _returnvalue))))

(fn `OffsetAllDecorations`
  (bind (_updatepos_x _updatepos_y) (`KismetMathLibrary.BreakVector` (`self.UpdatePos`)))
  (for _array_element (`self.GolfDecorations`)
    (`/Game/Blueprints/HoldableProps/Golf/BP_GolfDecorationBase.MoveActorRelativeToBall` _array_element (`KismetMathLibrary.MakeVector` _updatepos_x _updatepos_y))))

(fn `SetAllGolfDecorations`
  (bind _outactors (`GameplayStatics.GetAllActorsOfClass` "/Game/Blueprints/HoldableProps/Golf/BP_GolfDecorationBase.BP_GolfDecorationBase_C"))
  (set `self.GolfDecorations` _outactors))

(fn `UserConstructionScript`)