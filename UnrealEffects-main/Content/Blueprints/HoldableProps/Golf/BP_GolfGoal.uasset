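; BP_GolfGoal is a golf target that moves in response to the golf ball's goal-reached and goal-not-reached events.
; On success it turns green, waits two seconds, resets its color and jumps to a random reachable navigation point.
; On a miss it shifts horizontally by the inverse of the ball's displacement from start to final position, keeping its starting height.
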(event `UpdateOnGoalReached`
  (`MeshComponent.SetVectorParameterValueOnMaterials` (`self.StaticMesh`) "Color" (0.0 1.0 0.0))
  (`KismetSystemLibrary.Delay` 2.0)
  (`MeshComponent.SetVectorParameterValueOnMaterials` (`self.StaticMesh`) "Color" (0.0 1.0 0.87))
  (`SceneComponent.K2_SetWorldLocation` (`self.StaticMesh`) (`NavigationSystemV1.K2_GetRandomReachablePointInRadius` (0.0 0.0 0.0) 1500.0 null null) false false))

(event `self.ReceiveBeginPlay`
  (bind _golfball (`self.GolfBall`))
  (bind (_returnvalue_x _returnvalue_y _returnvalue_z) (`KismetMathLibrary.BreakVector` (`SceneComponent.K2_GetComponentLocation` (`self.StaticMesh`))))
  (add `/Game/Blueprints/HoldableProps/Golf/BP_RollingSphere.GolfGoalReached` _golfball (delegate `UpdateOnGoalReached`))
  (add `/Game/Blueprints/HoldableProps/Golf/BP_RollingSphere.GolfGoalNotReached` _golfball (delegate `UpdateGoalPos`))
  (set `self.StartingHeight` _returnvalue_z))

(event `UpdateGoalPos`
  (bind _staticmesh (`self.StaticMesh`))
  (bind (_returnvalue_x _returnvalue_y) (`KismetMathLibrary.BreakVector` (+ (`SceneComponent.K2_GetComponentLocation` _staticmesh) (`self.UpdatePos`))))
  (`self.GetBallDisplacement`)
  (`SceneComponent.K2_SetWorldLocation` _staticmesh (`KismetMathLibrary.MakeVector` _returnvalue_x _returnvalue_y (`self.StartingHeight`)) false false))

(fn `GetBallDisplacement`
  (bind _golfball (`self.GolfBall`))
  (set `self.UpdatePos` (* (- (`/Game/Blueprints/HoldableProps/Golf/BP_RollingSphere.FinalPos` _golfball) (`/Game/Blueprints/HoldableProps/Golf/BP_RollingSphere.StartingPos` _golfball)) -1.0)))

(fn `UserConstructionScript`)