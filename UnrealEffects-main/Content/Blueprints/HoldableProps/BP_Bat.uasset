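; BP_Bat is a holdable bat prop that shows a fire Niagara effect while it is swung quickly.
; Each tick it compares the Locator component's world position with the previous frame's and activates NSFire when the movement passes a fixed distance, deactivating it otherwise.
; The threshold is per frame, not scaled by delta time, so the effect depends on frame rate.
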(event `self.ReceiveBeginPlay`
  (`parent.ReceiveBeginPlay`)
  (set `self.LastFramePos` (`SceneComponent.K2_GetComponentLocation` (`self.Locator`))))

(event `self.ReceiveTick`
  (params (DeltaSeconds :type "Float (single-precision)"))
  (bind _ns_fire (`self.NS_Fire`))
  (bind _returnvalue (`SceneComponent.K2_GetComponentLocation` (`self.Locator`)))
  (if (>= (`KismetMathLibrary.VSize` (- _returnvalue (`self.LastFramePos`))) 15.0)
    (`ActorComponent.Activate` _ns_fire false)
    (else
      (`ActorComponent.Deactivate` _ns_fire)))
  (set `self.LastFramePos` _returnvalue))

(event `/Game/Blueprints/HoldableProps/GrippableInterface.OnDropped`
  (`parent.OnDropped`))

(fn `UserConstructionScript`)