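; Hand prop that automatically grips objects implementing GrippableInterface and releases them with a tilt-and-flick motion.
; Sphere overlap attaches one object at a time to the Hand, matches its rotation and sends OnGrippedMessage.
; Each Tick compares hand rotation to the previous frame; high pitch plus a sharp change detaches the object and sends OnDroppedMessage.
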(event `self.ReceiveBeginPlay`
  (set `self.StartingRotation` (`SceneComponent.K2_GetComponentRotation` (`self.Hand`))))

(event `self.ReceiveTick`
  (params (DeltaSeconds :type "Float (single-precision)"))
  (bind _grabbedactor (`self.GrabbedActor`))
  (set `self.CurrentRotation` (`SceneComponent.K2_GetComponentRotation` (`self.Hand`)))
  (bind _shoulddrop (`self.ShouldDrop`))
  (if _shoulddrop
    (if (`self.HasObjectGripped`)
      (`SceneComponent.K2_DetachFromComponent` (`Actor.RootComponent` _grabbedactor) "KeepWorld" "KeepRelative" "KeepWorld" true)
      (message `/Game/Blueprints/HoldableProps/GrippableInterface.OnDropped` _grabbedactor)
      (set `self.HasObjectGripped` false)
      (set `self.GrabbedActor` null))))

(event `self.Sphere.OnComponentBeginOverlap`
  (params (OverlappedComponent :type "PrimitiveComponent Object Reference") (OtherActor :type "Actor Object Reference") (OtherComp :type "PrimitiveComponent Object Reference") (OtherBodyIndex :type Integer) (bFromSweep :type Boolean) (SweepResult :type "HitResult Structure (by ref)"))
  (if (`KismetSystemLibrary.DoesImplementInterface` OtherActor "/Game/Blueprints/HoldableProps/GrippableInterface.GrippableInterface_C")
    (`/Engine/EditorBlueprintResources/StandardMacros.IsValid` (`self.GrabbedActor`)
      (:`Is Not Valid`
        (if (not (`self.HasObjectGripped`))
          (bind _output_get (set `self.GrabbedActor` OtherActor))
          (`self.GrabActor` _output_get)
          (set `self.HasObjectGripped` true))))))

(fn `GrabActor`
  (params (ActorToGrab :type "Actor Object Reference"))
  (`self.K2_AttachToComponent` ActorToGrab (`self.Hand`) "None" "SnapToTarget" "KeepWorld" "KeepWorld" true)
  (`self.K2_SetActorRotation` (`self.GrabbedActor`) (`SceneComponent.K2_GetComponentRotation` (`self.Hand`)) false)
  (message `/Game/Blueprints/HoldableProps/GrippableInterface.OnGripped` (`self.GrabbedActor`)))

(fn `ShouldDrop`
  (returns (ShouldDrop :type Boolean))
  (bind (_returnvalue_roll _returnvalue_pitch) (`KismetMathLibrary.BreakRotator` (`SceneComponent.K2_GetComponentRotation` (`self.Hand`))))
  (if (and (> _returnvalue_pitch 40.0) (> (`KismetMathLibrary.VSize` (- (`.Z` (`KismetMathLibrary.BreakRotIntoAxes` (`self.CurrentRotation`))) (`.Z` (`KismetMathLibrary.BreakRotIntoAxes` (`self.StartingRotation`))))) 0.38))
    (set `self.StartingRotation` (`self.CurrentRotation`))
    (return true)
    (else
      (set `self.StartingRotation` (`self.CurrentRotation`))
      (return false))))

(fn `UserConstructionScript`)