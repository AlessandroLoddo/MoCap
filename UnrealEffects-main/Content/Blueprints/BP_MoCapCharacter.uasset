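; BP_MoCapCharacter is a character that follows a spawned GrippingHand actor, apparently so its animated right hand stays on that hand.
; BeginPlay spawns the hand and records the mesh's starting height, which is not read afterwards.
; Each Tick offsets the actor from the hand by the spine_05-to-right-hand-grabber socket vector in X and Y, with fixed Z.
; Yaw matching to the hand is present but disconnected.
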(event `self.ReceiveBeginPlay`
  (bind (_returnvalue_x _returnvalue_y _returnvalue_z) (`KismetMathLibrary.BreakVector` (`SceneComponent.K2_GetComponentLocation` (`self.Mesh`))))
  (set `self.StartingZPos` _returnvalue_z)
  (bind _returnvalue (`|SpawnActorFromClass` "/Game/Blueprints/Props/Misc/GrippingHand.GrippingHand_C" (`KismetMathLibrary.MakeTransform` (0.0 0.0 0.0)) "Undefined" "MultiplyWithRoot" null null))
  (set `self.Hand` _returnvalue))

(event `self.ReceiveTick`
  (params (DeltaSeconds :type "Float (single-precision)"))
  (bind _returnvalue_location (`KismetMathLibrary.BreakTransform` (`SceneComponent.GetSocketTransform` (`self.Mesh`) "spine_05" "RTS_World")))
  (bind _returnvalue_location_2 (`KismetMathLibrary.BreakTransform` (`SceneComponent.GetSocketTransform` (`self.Mesh`) "hand_r_Grabber_socket" "RTS_World")))
  (bind (_returnvalue_x _returnvalue_y) (`KismetMathLibrary.BreakVector` (+ (`self.K2_GetActorLocation` (stale `self.ReceiveBeginPlay` _returnvalue)) (- _returnvalue_location _returnvalue_location_2))))
  (`self.K2_SetActorLocation` self (`KismetMathLibrary.MakeVector` _returnvalue_x _returnvalue_y 90.0) false false))

(fn `UserConstructionScript`)