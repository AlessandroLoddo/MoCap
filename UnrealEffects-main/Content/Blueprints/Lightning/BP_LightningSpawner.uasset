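; Lightning spawner actor that throws Niagara lightning beams at a BP_Axe once the axe overlaps its Range component.
; The overlap caches the axe and starts an endless loop that attaches a new NS_FusionSystem to Sphere at random sub-second intervals.
; Each beam's Beam_End is set to the axe's LightningReceiver location at spawn.
; Ending overlap with Sphere, rather than Range, clears the axe reference but leaves the loop running.
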(event `LightningSpawn`
  (bind _returnvalue (`NiagaraFunctionLibrary.SpawnSystemAttached` "/Game/VisualEffects/NS_FusionSystem.NS_FusionSystem" (`self.Sphere`) "None" (0.0 0.0 0.0) (struct) "KeepRelativeOffset"))
  (`NiagaraComponent.SetVariableVec3` _returnvalue "Beam_End" (`SceneComponent.K2_GetComponentLocation` (`/Game/Blueprints/HoldableProps/BP_Axe.LightningReceiver` (`self.Axe`)))))

(event `self.Range.OnComponentBeginOverlap`
  (params (OverlappedComponent :type "PrimitiveComponent Object Reference") (OtherActor :type "Actor Object Reference") (OtherComp :type "PrimitiveComponent Object Reference") (OtherBodyIndex :type Integer) (bFromSweep :type Boolean) (SweepResult :type "HitResult Structure (by ref)"))
  (bind _asbp_axe (cast `/Game/Blueprints/HoldableProps/BP_Axe` OtherActor))
  (set `self.Axe` _asbp_axe)
  (`self.LightningSpawn` :!label _label)
  (`KismetSystemLibrary.Delay` (`KismetMathLibrary.RandomFloatInRange` 0.0 0.6))
  (goto _label))

(event `SpawnEffect`)

(event `self.Sphere.OnComponentEndOverlap`
  (params (OverlappedComponent :type "PrimitiveComponent Object Reference") (OtherActor :type "Actor Object Reference") (OtherComp :type "PrimitiveComponent Object Reference") (OtherBodyIndex :type Integer))
  (set `self.Axe` null))

(fn `UserConstructionScript`)