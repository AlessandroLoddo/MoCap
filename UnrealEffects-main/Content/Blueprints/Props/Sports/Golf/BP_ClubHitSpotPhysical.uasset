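; Physical collision proxy for the golf club head, kept separate from the club to avoid rotation and collision issues.
; On BeginPlay it finds the first BP_GolfClub in the level.
; Each tick it moves its Sphere to the club's ClubHitSpot world location without sweep or teleport, setting world rotation from that spot's relative rotation.
; The author flags this per-tick follow as a disliked but workable workaround.
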(event `self.ReceiveBeginPlay`
  (bind _outactors (`GameplayStatics.GetAllActorsOfClass` "/Game/Blueprints/Props/Sports/Golf/BP_GolfClub.BP_GolfClub_C"))
  (set `self.Club` (`|GetArrayItem` _outactors)))

(event `self.ReceiveTick`
  (params (DeltaSeconds :type "Float (single-precision)"))
  (bind _sphere (`self.Sphere`))
  (bind _clubhitspot (`/Game/Blueprints/Props/Sports/Golf/BP_GolfClub.ClubHitSpot` (`self.Club`)))
  (bind (_returnvalue_location _returnvalue_rotation) (`KismetMathLibrary.BreakTransform` (`SceneComponent.GetRelativeTransform` _clubhitspot)))
  ;[1 0 0.7207] I hate this implementation but it is a viable way to provide collision to the end of the club without having rotation/collision issues
  (`SceneComponent.K2_SetWorldLocation` _sphere (`SceneComponent.K2_GetComponentLocation` _clubhitspot) false false)
  (`SceneComponent.K2_SetWorldRotation` _sphere _returnvalue_rotation false false))

(fn `UserConstructionScript`)