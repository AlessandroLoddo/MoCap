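; Golf hole goal actor with a height indicator animated by a looping timeline until the goal is reached, also restarted by the ball's update event.
; On victory it flashes the hole green, relocates to a random reachable nav point after a delay, and resets the ball.
; Helper functions store ball displacement and position the pawn camera behind and above the ball, while club rotation is an unfinished stub.
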(event `Indicator Movement`
  (bind _indicator (`self.Indicator`))
  (bind (_returnvalue_x _returnvalue_y) (`KismetMathLibrary.BreakVector` (`SceneComponent.K2_GetComponentLocation` _indicator)))
  (bind (_direction _newtrack_0) (`Timeline|IndicatorTimeline` :!via `PlayFromStart` :!label _label)
    (:`Update`
      (if (not (`self.WasGoalReached`))
        (bind _returnvalue (+ (`self.UpdateHeightIndicator`) _newtrack_0))
        (`SceneComponent.K2_SetWorldLocation` _indicator (`KismetMathLibrary.MakeVector` _returnvalue_x _returnvalue_y _returnvalue) false false)
        (set `self.UpdateHeightIndicator` _returnvalue)))
    (:`Finished`
      (`KismetSystemLibrary.Delay` 0.001)
      (goto _label :!via `PlayFromStart`))))

(event `self.ReceiveBeginPlay`
  (bind (_returnvalue_x _returnvalue_y _returnvalue_z) (`KismetMathLibrary.BreakVector` (`SceneComponent.K2_GetComponentLocation` (`self.Indicator`))))
  (set `self.StartingHeightIndicator` _returnvalue_z)
  (set `self.UpdateHeightIndicator` (`self.StartingHeightIndicator`))
  (`self.Indicator Movement`)
  (add `/Game/Blueprints/Props/Sports/Golf/BP_RollingSphere.UpdateBall` (`self.GolfBall`) (delegate `Indicator Movement`)))

(event `DisplayVictory`
  (set `self.WasGoalReached` true)
  (`MeshComponent.SetVectorParameterValueOnMaterials` (`self.Hole`) "Color" (0.0 1.0 0.0))
  (`KismetSystemLibrary.Delay` 2.0)
  (`MeshComponent.SetVectorParameterValueOnMaterials` (`self.Hole`) "Color" (0.0 1.0 0.87))
  (`SceneComponent.K2_SetWorldLocation` (`self.DefaultSceneRoot`) (`NavigationSystemV1.K2_GetRandomReachablePointInRadius` (0.0 0.0 -24.041572) 1500.0 null null) false false)
  (`self.Indicator Movement`)
  (`/Game/Blueprints/Props/Sports/Golf/BP_RollingSphere.ResetBall` (`self.GolfBall`))
  (set `self.WasGoalReached` false))

(fn `ApplyCameraOffset`
  (bind _sphere (`/Game/Blueprints/Props/Sports/Golf/BP_RollingSphere.Sphere` (`self.GolfBall`)))
  (bind _returnvalue (`SceneComponent.K2_GetComponentLocation` _sphere))
  (bind (_returnvalue_x _returnvalue_y _returnvalue_z) (`KismetMathLibrary.BreakVector` (+ _returnvalue (/ 1000.0 4.0))))
  (bind (_returnvalue_x_2 _returnvalue_y_2) (`KismetMathLibrary.BreakVector` (+ _returnvalue (* (* (`SceneComponent.GetForwardVector` _sphere) -1.0) 400.0))))
  (`SceneComponent.K2_SetWorldLocation` (`/Game/Blueprints/BP_MoCapPawn.Camera` (`self.MyPawn`)) (`KismetMathLibrary.MakeVector` _returnvalue_x_2 _returnvalue_y_2 _returnvalue_z) false false))

(fn `ApplyClubRotation`)

(fn `GetBallDisplacement`
  (bind _golfball (`self.GolfBall`))
  (bind _returnvalue (- (`SceneComponent.K2_GetComponentLocation` (`/Game/Blueprints/Props/Sports/Golf/BP_RollingSphere.Sphere` _golfball)) (`/Game/Blueprints/Props/Sports/Golf/BP_RollingSphere.StartingPos` _golfball)))
  (set `self.UpdatePos` (* (`KismetMathLibrary.Normal` _returnvalue) (`KismetMathLibrary.VSize` _returnvalue))))

(fn `SetWasScoreReached`
  (params (Val :type Boolean))
  (set `self.WasGoalReached` Val))

(fn `UserConstructionScript`)