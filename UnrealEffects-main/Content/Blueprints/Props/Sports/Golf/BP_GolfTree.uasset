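; BP_GolfTree is a golf prop Blueprint that shows a randomly chosen tree when play begins.
; On BeginPlay, InitialiseMeshes gathers three tree components into an array and makes one at a random index visible.
; It only ever turns visibility on, and the construction script adds nothing beyond the parent call, so the pick happens at runtime.
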(event `self.ReceiveBeginPlay`
  (`parent.ReceiveBeginPlay`)
  (`self.InitialiseMeshes`))

(fn `InitialiseMeshes`
  (bind _output_get (set `self.Meshes` (`|MakeArray` (`self.Tree1`) (`self.Tree2`) (`self.Tree3`))))
  (`SceneComponent.SetVisibility` (`|GetArrayItem` _output_get (`KismetMathLibrary.RandomIntegerInRange` 0 2)) true false))

(fn `UserConstructionScript`
  (`parent.UserConstructionScript`))