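; BP_BallSpawner is a baseball launcher prop that repeatedly throws balls in an arc.
; A Tick-driven timer spawns a BP_Baseball at the actor's transform every two seconds.
; Each ball's Sphere receives a randomized velocity along the StaticMesh's forward and up vectors, so throws follow the mesh's facing with slight variation, plus a fixed angular velocity for spin.
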(event `self.ReceiveTick`
  (params (DeltaSeconds :type "Float (single-precision)"))
  (bind _staticmesh (`self.StaticMesh`))
  (bind _output_get (set `self.SpawnTimer` (+ (`self.SpawnTimer`) DeltaSeconds)))
  (if (>= _output_get 2.0)
    (set `self.SpawnTimer` 0.0)
    (bind _returnvalue (`|SpawnActorFromClass` "/Game/Blueprints/Props/Sports/Baseball/BP_Baseball.BP_Baseball_C" (`self.GetTransform` self) "Undefined" "MultiplyWithRoot" null null))
    (bind _sphere (`/Game/Blueprints/Props/Sports/Baseball/BP_Baseball.Sphere` _returnvalue))
    (`GeometryCollectionComponent.ApplyLinearVelocity` _sphere 0 (+ (* (`SceneComponent.GetForwardVector` _staticmesh) (`KismetMathLibrary.RandomFloatInRange` 750.0 810.0)) (* (`SceneComponent.GetUpVector` _staticmesh) (`KismetMathLibrary.RandomFloatInRange` 450.0 510.0))))
    (`GeometryCollectionComponent.ApplyAngularVelocity` _sphere 0 (20.0 30.0 0.0))))

(fn `UserConstructionScript`)