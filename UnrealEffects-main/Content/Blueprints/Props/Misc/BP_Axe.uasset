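; BP_Axe is a grippable axe prop that shows a fire effect while it is swung or moved.
; While gripped, Tick compares the mesh's world position to the previous frame's against a fixed per-frame distance threshold, using absolute-value vectors.
; Movement lazily spawns NS_TorchFire on LightningReceiver, then reactivates that cached Niagara component.
; Slowing below the threshold or dropping the axe deactivates the effect.
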(event `self.ReceiveBeginPlay`
  (set `self.Character` (`GameplayStatics.GetPlayerCharacter` 0))
  (`parent.ReceiveBeginPlay`)
  (set `self.PreviousPos` (`SceneComponent.K2_GetComponentLocation` (`self.GrippableObjectMesh`))))

(event `/Game/Blueprints/Props/GrippableInterface.OnDropped`
  (bind _particleeffect (`self.ParticleEffect`))
  (`parent.OnDropped`)
  (if (`KismetSystemLibrary.IsValid` _particleeffect)
    (`ActorComponent.Deactivate` _particleeffect)))

(event `/Game/Blueprints/Props/GrippableInterface.OnGripped`
  (`parent.OnGripped`))

(event `self.ReceiveTick`
  (params (DeltaSeconds :type "Float (single-precision)"))
  (if (`self.bIsGripped`)
    (set `self.CurrentPos` (`SceneComponent.K2_GetComponentLocation` (`self.GrippableObjectMesh`)))
    (`self.CheckForSpeed`)
    (set `self.PreviousPos` (`self.CurrentPos`))))

(fn `CheckForSpeed`
  (bind _particleeffect (`self.ParticleEffect`))
  (bind _particleeffect_2 (`self.ParticleEffect`))
  (bind _isfast (`self.IsMoving`))
  (if _isfast
    (`/Engine/EditorBlueprintResources/StandardMacros.IsValid` _particleeffect_2
      (:`Is Valid`
        (`ActorComponent.Activate` _particleeffect_2 false))
      (:`Is Not Valid`
        (bind _returnvalue (`NiagaraFunctionLibrary.SpawnSystemAttached` "/Game/VisualEffects/NS_TorchFire.NS_TorchFire" (`self.LightningReceiver`) "Scene" (0.0 0.0 0.0) (`KismetMathLibrary.MakeRotator` 0.0) "SnapToTargetIncludingScale"))
        (set `self.ParticleEffect` _returnvalue)))
    (else
      (`/Engine/EditorBlueprintResources/StandardMacros.IsValid` _particleeffect
        (:`Is Valid`
          (`ActorComponent.Deactivate` _particleeffect))))))

(fn `IsMoving`
  (returns (IsFast :type Boolean))
  (if (> (`KismetMathLibrary.VSize` (- (`KismetMathLibrary.Vector_GetAbs` (`self.PreviousPos`)) (`KismetMathLibrary.Vector_GetAbs` (`self.CurrentPos`)))) 0.8)
    (return true)
    (else
      (return false))))

(fn `UserConstructionScript`)