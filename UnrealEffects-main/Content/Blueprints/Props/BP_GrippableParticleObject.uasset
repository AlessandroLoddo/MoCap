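; BP_GrippableParticleObject is a grippable prop that shows a particle effect while it is held.
; It extends its parent's grip events, activating the Particles component on grip without a reset and deactivating it on drop.
; BeginPlay and the construction script only call the parent, and Tick and overlap events are disabled.
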(event `self.ReceiveBeginPlay`
  (`parent.ReceiveBeginPlay`))

(event `/Game/Blueprints/Props/GrippableInterface.OnDropped`
  (`parent.OnDropped`)
  (`ActorComponent.Deactivate` (`self.Particles`)))

(event `/Game/Blueprints/Props/GrippableInterface.OnGripped`
  (`parent.OnGripped`)
  (`ActorComponent.Activate` (`self.Particles`) false))

(fn `UserConstructionScript`
  (`parent.UserConstructionScript`))