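; Cannon prop that a grippable lighter both fires and aims, depending on how the lighter is held.
; A tilted lighter entering the Sphere spawns a CannonBall, launched along FireLocation's negated forward vector, then starts a short cooldown counted on Tick.
; While a vertical lighter overlaps the Sphere, Tick adds its frame-to-frame Z rotation change to CannonBase's yaw, ignoring tiny changes.
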(event `self.ReceiveBeginPlay`
  (`self.K2_AttachToComponent` (`self.MainCamera`) (`self.CannonBase`) "None" "KeepWorld" "KeepWorld" "KeepWorld" true))

(event `ShootBall`
  (bind _returnvalue (`|SpawnActorFromClass` "/Game/Blueprints/Props/Cannon/CannonBall.CannonBall_C" (`KismetMathLibrary.MakeTransform` (`SceneComponent.K2_GetComponentLocation` (`self.FireLocation`))) "Undefined" "MultiplyWithRoot" null null))
  (`PrimitiveComponent.SetPhysicsLinearVelocity` (`/Game/Blueprints/Props/BP_BaseGrippableObject.GrippableObjectMesh` _returnvalue) (* (* (`SceneComponent.GetForwardVector` (`self.FireLocation`)) (-1.0 -1.0 -1.0)) (`/Game/Blueprints/Props/Cannon/CannonBall.GetShootSpeed` _returnvalue)) false "None"))

(event `self.Sphere.OnComponentBeginOverlap`
  (params (OverlappedComponent :type "PrimitiveComponent Object Reference") (OtherActor :type "Actor Object Reference") (OtherComp :type "PrimitiveComponent Object Reference") (OtherBodyIndex :type Integer) (bFromSweep :type Boolean) (SweepResult :type "HitResult Structure (by ref)"))
  (cast `/Game/Blueprints/Props/Cannon/BP_CannonLighter` OtherActor)
  (if (`self.InCooldown`)
    _
    (elif (not (`self.IsLighterVertical`))
      (`self.ShootBall`)
      (set `self.InCooldown` true)
      (set `self.CooldownTimer` 0.0))))

(event `self.ReceiveTick`
  (params (DeltaSeconds :type "Float (single-precision)"))
  (`|ExecutionSequence`
    (:`then_0`
      (`self.TimerUpdate`))
    (:`then_1`
      (`self.RotateInRange`))))

(event `self.Sphere.OnComponentEndOverlap`
  (params (OverlappedComponent :type "PrimitiveComponent Object Reference") (OtherActor :type "Actor Object Reference") (OtherComp :type "PrimitiveComponent Object Reference") (OtherBodyIndex :type Integer)))

(fn `HasCannonLighterMoved`
  (returns (ReturnValue :type Boolean))
  (bind _cannonlighter (`self.CannonLighter`))
  (bind _returnvalue (- (`/Game/Blueprints/Props/Cannon/BP_CannonLighter.CurrentZRot` _cannonlighter) (`/Game/Blueprints/Props/Cannon/BP_CannonLighter.PreviousZRot` _cannonlighter)))
  (`KismetSystemLibrary.PrintString` "Hello")
  (return (or (< _returnvalue -0.1) (> _returnvalue 0.1))))

(fn `IsLighterVertical`
  (returns (IsLighterVertical :type Boolean))
  (bind (_returnvalue_roll _returnvalue_pitch) (`KismetMathLibrary.BreakRotator` (`SceneComponent.K2_GetComponentRotation` (`/Game/Blueprints/Props/BP_BaseGrippableObject.GrippableObjectMesh` (`self.CannonLighter`)))))
  (return (and (< _returnvalue_roll 13.0) (< _returnvalue_pitch 13.0))))

(fn `RotateInRange`
  (bind _cannonlighter (`self.CannonLighter`))
  (bind _cannonbase (`self.CannonBase`))
  (bind _cannonlighter_2 (`self.CannonLighter`))
  (bind (_returnvalue_roll _returnvalue_pitch _returnvalue_yaw) (`KismetMathLibrary.BreakRotator` (`SceneComponent.K2_GetComponentRotation` _cannonbase)))
  (if (!= (`KismetArrayLibrary.Array_Find` (`PrimitiveComponent.GetOverlappingActors` (`self.Sphere`) "/Game/Blueprints/Props/Cannon/BP_CannonLighter.BP_CannonLighter_C") (`self.CannonLighter`)) -1)
    (if (`self.IsLighterVertical`)
      (if (`self.HasCannonLighterMoved`)
        (if (`self.isFirstRot`)
          (set `self.isFirstRot` false)
          (else
            ;[1 1 1] Set cannon rotation to be same as lighter rotation
            (`SceneComponent.K2_SetWorldRotation` _cannonbase (`KismetMathLibrary.MakeRotator` _returnvalue_roll _returnvalue_pitch (+ _returnvalue_yaw (- (`/Game/Blueprints/Props/Cannon/BP_CannonLighter.CurrentZRot` _cannonlighter_2) (`/Game/Blueprints/Props/Cannon/BP_CannonLighter.PreviousZRot` _cannonlighter_2)))) false false))))))
  ;[1 0.1114 0] Set previous Z rotation for calculating rotation difference between frames
  (set `/Game/Blueprints/Props/Cannon/BP_CannonLighter.PreviousZRot` (`/Game/Blueprints/Props/Cannon/BP_CannonLighter.CurrentZRot` _cannonlighter) _cannonlighter))

(fn `TimerUpdate`
  (if (`self.InCooldown`)
    (bind _output_get (set `self.CooldownTimer` (+ (`self.CooldownTimer`) (`GameplayStatics.GetWorldDeltaSeconds`))))
    (if (> _output_get 3.0)
      (set `self.InCooldown` false))))

(fn `UserConstructionScript`)