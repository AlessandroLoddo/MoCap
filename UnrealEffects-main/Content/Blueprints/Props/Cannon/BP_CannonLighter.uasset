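; BP_CannonLighter is a cannon lighter prop that extends a parent class providing GrippableObjectMesh.
; On BeginPlay it seeds current, previous and applied rotation variables from the mesh's world yaw.
; Tick refreshes only the current yaw, and nothing in this graph acts on the values.
; A debug print of previous and current yaw is left unconnected, and the construction script only calls the parent.
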(event `self.ReceiveBeginPlay`
  (bind (_returnvalue_roll _returnvalue_pitch _returnvalue_yaw) (`KismetMathLibrary.BreakRotator` (`SceneComponent.K2_GetComponentRotation` (`self.GrippableObjectMesh`))))
  (`parent.ReceiveBeginPlay`)
  (set `self.CurrentZRot` _returnvalue_yaw)
  (set `self.PreviousZRot` _returnvalue_yaw)
  (set `self.AppliedRot` _returnvalue_yaw))

(event `self.ReceiveTick`
  (params (DeltaSeconds :type "Float (single-precision)"))
  (bind (_returnvalue_roll _returnvalue_pitch _returnvalue_yaw) (`KismetMathLibrary.BreakRotator` (`SceneComponent.K2_GetComponentRotation` (`self.GrippableObjectMesh`))))
  (`parent.ReceiveTick` DeltaSeconds)
  (set `self.CurrentZRot` _returnvalue_yaw))

(fn `UserConstructionScript`
  (`parent.UserConstructionScript`))