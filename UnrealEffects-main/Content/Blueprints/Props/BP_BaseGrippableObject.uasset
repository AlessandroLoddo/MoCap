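; BP_BaseGrippableObject is a base prop actor for objects that can be gripped, returning to its starting placement when dropped.
; On BeginPlay it stores the root component's world transform as StartingTransform.
; OnGripped sets the IsGripped flag; OnDropped clears it and snaps the actor back to that stored transform.
; A separate ResetPosition function performs the same transform restore on demand.
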(event `self.ReceiveBeginPlay`
  (set `self.StartingTransform` (`SceneComponent.K2_GetComponentToWorld` (`self.DefaultSceneRoot`))))

(event `self.ReceiveTick`
  (params (DeltaSeconds :type "Float (single-precision)")))

(event `/Game/Blueprints/Props/GrippableInterface.OnDropped`
  (`self.K2_SetActorTransform` (`self.StartingTransform`))
  (set `self.bIsGripped` false))

(event `/Game/Blueprints/Props/GrippableInterface.OnGripped`
  (set `self.bIsGripped` true))

(fn `ResetPosition`
  (`self.K2_SetActorTransform` (`self.StartingTransform`)))

(fn `UserConstructionScript`)