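; BP_BallSpawner is a baseball launcher that spawns a BP_Baseball at its own transform every two seconds.
; Tick accumulates a timer, then gives each new ball's sphere a randomized velocity along the static mesh's forward and up vectors, producing a lobbed pitch.
; It also applies a random spin around the up vector.
; Tick prints the mesh's forward vector to screen every frame as debug output.
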(event `self.ReceiveTick`
  (params (DeltaSeconds :type "Float (single-precision)"))
  (bind _staticmesh (`self.StaticMesh`))
  (bind _returnvalue (* (`SceneComponent.GetUpVector` _staticmesh) (`KismetMathLibrary.RandomFloatInRange` 450.0 510.0)))
  (`KismetSystemLibrary.PrintString` (`KismetStringLibrary.Conv_VectorToString` (`SceneComponent.GetForwardVector` (`self.StaticMesh`))))
  (bind _output_get (set `self.SpawnTimer` (+ (`self.SpawnTimer`) DeltaSeconds)))
  (if (>= _output_get 2.0)
    (set `self.SpawnTimer` 0.0)
    (bind _returnvalue_2 (`|SpawnActorFromClass` "/Game/Blueprints/Baseball/BP_Baseball.BP_Baseball_C" (`self.GetTransform` self) "Undefined" "MultiplyWithRoot" null null))
    (bind _sphere (`/Game/Blueprints/Baseball/BP_Baseball.Sphere` _returnvalue_2))
    (`GeometryCollectionComponent.ApplyLinearVelocity` _sphere 0 (+ (* (`SceneComponent.GetForwardVector` _staticmesh) (`KismetMathLibrary.RandomFloatInRange` 750.0 810.0)) _returnvalue))
    (`GeometryCollectionComponent.ApplyAngularVelocity` _sphere 0 _returnvalue)))

(fn `UserConstructionScript`)